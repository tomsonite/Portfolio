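; BP_Target is a hittable target that briefly activates a receiver when struck.
; HitTarget, behind a resettable DoOnce, activates the receiver, plays an unlock sound and tilts the Scene component via a timeline.
; After a short delay a second timeline restores it, deactivates the receiver and re-arms the target.
; Sphere overlap passes the target to the overlapping actor through ActivateTargetMessage; HitTarget has no caller here.
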(event `HitTarget`
  (`/Engine/EditorBlueprintResources/StandardMacros.DoOnce` false :!label _label
    (:`Completed`
      (`self.ActivateReceiver`)
      (`GameplayStatics.SpawnSoundAttached` "/Game/MyContent/Sounds/SW_Unlocked.SW_Unlocked" (`self.DefaultSceneRoot`) "None" (0.0 0.0 0.0) (struct) "KeepRelativeOffset" false 1.0 1.0 0.0 "/Game/MyContent/Sounds/Att_Object.Att_Object" null)
      (bind (_direction _newtrack_0) (`Timeline|Timeline_0` :!via `PlayFromStart`)
        (:`Update`
          (`SceneComponent.K2_SetRelativeRotation` (`self.scene`) (`KismetMathLibrary.RLerp` (struct) (struct :`Roll` -40.0) _newtrack_0) false false))
        (:`Finished`
          (`KismetSystemLibrary.Delay` 1.0)
          (bind (_direction_2 _newtrack_0_2) (`Timeline|Timeline_1` :!via `PlayFromStart`)
            (:`Update`
              (`SceneComponent.K2_SetRelativeRotation` (`self.scene`) (`KismetMathLibrary.RLerp` (struct :`Roll` -40.0) (struct) _newtrack_0_2) false false))
            (:`Finished`
              (`self.DeactivateReceiver`)
              (goto _label :!via `Reset`))))))))

(event `self.Sphere.OnComponentBeginOverlap`
  (params (OverlappedComponent :type "PrimitiveComponent Object Reference") (OtherActor :type "Actor Object Reference") (OtherComp :type "PrimitiveComponent Object Reference") (OtherBodyIndex :type Integer) (bFromSweep :type Boolean) (SweepResult :type "HitResult Structure (by ref)"))
  (message `/Game/MyContent/Blueprints/Interfaces/BPI_PhysicsObject.ActivateTarget` OtherActor self))

(event `self.Sphere.OnComponentEndOverlap`
  (params (OverlappedComponent :type "PrimitiveComponent Object Reference") (OtherActor :type "Actor Object Reference") (OtherComp :type "PrimitiveComponent Object Reference") (OtherBodyIndex :type Integer)))

(fn `UserConstructionScript`
  (`parent.UserConstructionScript`))