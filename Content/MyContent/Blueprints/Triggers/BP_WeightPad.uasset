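; BP_WeightPad is a pressure pad trigger that sinks and rises to switch a receiver on and off.
; On box begin and end overlap, it messages the other actor with itself, leaving that actor to decide whether to trigger the pad.
; ActivatePad uses a FlipFlop to alternately play and reverse a timeline lowering Cube1.
; When the timeline finishes, its direction selects ActivateReceiver or DeactivateReceiver.
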(event `ActivatePad`
  (`/Engine/EditorBlueprintResources/StandardMacros.FlipFlop`
    (:`A`
      (bind (_direction _newtrack_0) (`Timeline|Timeline_0` :!label _label)
        (:`Update`
          (`SceneComponent.K2_SetRelativeLocation` (`self.Cube1`) (`KismetMathLibrary.VLerp` (0.0 0.0 91.662712) (0.0 0.0 0.12) _newtrack_0) false false))
        (:`Finished`
          (switch `ETimelineDirection` _direction
            (:`Forward`
              (`self.ActivateReceiver`))
            (:`Backward`
              (`self.DeactivateReceiver`))))))
    (:`B`
      (goto _label :!via `Reverse`))))

(event `self.Box.OnComponentBeginOverlap`
  (params (OverlappedComponent :type "PrimitiveComponent Object Reference") (OtherActor :type "Actor Object Reference") (OtherComp :type "PrimitiveComponent Object Reference") (OtherBodyIndex :type Integer) (bFromSweep :type Boolean) (SweepResult :type "HitResult Structure (by ref)"))
  (message `/Game/MyContent/Blueprints/Interfaces/BPI_PhysicsObject.ActivateWeightPad` OtherActor self))

(event `self.Box.OnComponentEndOverlap`
  (params (OverlappedComponent :type "PrimitiveComponent Object Reference") (OtherActor :type "Actor Object Reference") (OtherComp :type "PrimitiveComponent Object Reference") (OtherBodyIndex :type Integer))
  (message `/Game/MyContent/Blueprints/Interfaces/BPI_PhysicsObject.ActivateWeightPad` OtherActor self))

(fn `UserConstructionScript`
  (`parent.UserConstructionScript`))