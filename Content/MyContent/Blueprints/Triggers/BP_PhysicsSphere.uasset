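; BP_PhysicsSphere is a physics object that the FPS character can grab, drop and throw, and that can activate targets.
; Interacting toggles between grabbing through the character's PhysicsHandle and releasing, adjusting angular damping and the throw tip UI.
; ApplyForce releases the sphere and applies a strong impulse away from the supplied location.
; ActivateTarget calls HitTarget on the target only while the sphere is not held.
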(event `/Game/MyContent/Blueprints/Interfaces/BPI_Interact.InteractWith`
  (params (FPS_Character :type "/Game/MyContent/Blueprints/Player/FirstPersonCharacter Object Reference"))
  (if (`self.IsGrabbed`)
    (`self.ReleaseObject` FPS_Character)
    (else
      (`self.GrabObject` FPS_Character))))

(event `/Game/MyContent/Blueprints/Interfaces/BPI_PhysicsObject.ActivateTarget`
  (params (Target :type "/Game/MyContent/Blueprints/Triggers/BP_Target Object Reference"))
  (if (not (`self.IsGrabbed`))
    (`/Game/MyContent/Blueprints/Triggers/BP_Target.HitTarget` Target)))

(event `/Game/MyContent/Blueprints/Interfaces/BPI_PhysicsObject.ApplyForce`
  (params (ActorLocation :type "Vector Structure") (FPS_Character :type "/Game/MyContent/Blueprints/Player/FirstPersonCharacter Object Reference"))
  (`self.ReleaseObject` FPS_Character)
  (`PrimitiveComponent.AddImpulse` (`self.StaticMesh`) (* (`KismetMathLibrary.Normal` (- (`SceneComponent.K2_GetComponentLocation` (`self.StaticMesh`)) ActorLocation)) 400000.0) "None" false))

(fn `GrabObject`
  (params (self2 :type "/Game/MyContent/Blueprints/Player/FirstPersonCharacter Object Reference"))
  (bind _staticmesh (`self.StaticMesh`))
  (`PhysicsHandleComponent.GrabComponentAtLocation` (`/Game/MyContent/Blueprints/Player/FirstPersonCharacter.PhysicsHandle` self2) _staticmesh "None" (`SceneComponent.K2_GetComponentLocation` _staticmesh))
  (`PrimitiveComponent.SetAngularDamping` (`self.StaticMesh`) 100.0)
  (set `self.IsGrabbed` true)
  (`/Game/MyContent/Blueprints/Player/FirstPersonCharacter.ToggleThrowTipUI` (`local.self2`) true))

(fn `ReleaseObject`
  (params (FPS_Character :type "/Game/MyContent/Blueprints/Player/FirstPersonCharacter Object Reference"))
  (`PhysicsHandleComponent.ReleaseComponent` (`/Game/MyContent/Blueprints/Player/FirstPersonCharacter.PhysicsHandle` FPS_Character))
  (`PrimitiveComponent.SetAngularDamping` (`self.StaticMesh`) 0.0)
  (set `self.IsGrabbed` false)
  (`/Game/MyContent/Blueprints/Player/FirstPersonCharacter.ToggleThrowTipUI` (`local.FPS_Character`) false))

(fn `UserConstructionScript`)