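; BP_Button is an interactive trigger button that the FPS character presses to switch a receiver on temporarily.
; Interactwith plays a click, activates the receiver and, if AddScore is set, calls CommunicateToMessage on the character.
; A timeline lerps the Cylinder's relative location to animate the press, then deactivates the receiver when finished.
; CanPress blocks repeat presses until the timeline ends.
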(event `/Game/MyContent/Blueprints/Interfaces/BPI_Interact.InteractWith`
  (params (FPS_Character :type "/Game/MyContent/Blueprints/Player/FirstPersonCharacter Object Reference"))
  (if (`self.CanPress`)
    (if (`self.AddScore?`)
      (message `/Game/MyContent/Blueprints/Interfaces/BPI_Interact.CommunicateTo` FPS_Character))
    (`GameplayStatics.PlaySoundAtLocation` "/Engine/VREditor/Sounds/UI/Click_on_Button_Cue.Click_on_Button_Cue" (`self.K2_GetActorLocation`) (struct) 1.0 1.0 0.0 "/Game/MyContent/Sounds/Att_Object.Att_Object" null null null)
    (`self.ActivateReceiver`)
    (set `self.CanPress` false)
    (bind (_direction _newtrack_0) (`Timeline|Timeline_0` :!via `PlayFromStart`)
      (:`Update`
        (`SceneComponent.K2_SetRelativeLocation` (`self.Cylinder`) (`KismetMathLibrary.VLerp` (3.830224 0.0 111.786064) (0.616288 0.0 107.955841) _newtrack_0) false false))
      (:`Finished`
        (set `self.CanPress` true)
        (`self.DeactivateReceiver`)))))

(fn `UserConstructionScript`)