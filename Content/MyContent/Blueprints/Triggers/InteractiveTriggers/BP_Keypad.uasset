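; Interactive keypad trigger that activates a receiver when the player enters the correct four-digit combination.
; Interaction matches the character's hit component to one of nine buttons, animates its press on a timeline and records the digit.
; The display updates until unlocked; every fourth digit triggers a combination check.
; Success turns the light green and stays unlocked; failure flashes red and briefly blocks input before resetting, each with its own sound.
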(event `/Game/MyContent/Blueprints/Interfaces/BPI_Interact.InteractWith`
  (params (FPS_Character :type "/Game/MyContent/Blueprints/Player/FirstPersonCharacter Object Reference"))
  (`self.OnButtonPressed` FPS_Character))

(event `OnButtonPressed`
  (params (FPS_Character :type "/Game/MyContent/Blueprints/Player/FirstPersonCharacter Object Reference"))
  ;[1 1 1] On button pressed
  (for (_array_element _array_index) (`|MakeArray` (`self.1`) (`self.2`) (`self.3`) (`self.4`) (`self.5`) (`self.6`) (`self.7`) (`self.8`) (`self.9`))
    (if (and (== _array_element (`/Game/MyContent/Blueprints/Player/FirstPersonCharacter.Hit Component` FPS_Character)) (`self.CanPressButton`) (not (`self.Locked`)))
      (switch `int` _array_index
        (:`0`
          (`self.AnimateButton` (`self.1`) (-12.152973 61.283737 -27.200123))
          (`self.EnterDigit` "1"))
        (:`1`
          (`self.AnimateButton` (`self.2`) (-12.153018 61.283646 0.0))
          (`self.EnterDigit` "2"))
        (:`2`
          (`self.AnimateButton` (`self.3`) (-12.153064 61.283543 27.199879))
          (`self.EnterDigit` "3"))
        (:`3`
          (`self.AnimateButton` (`self.4`) (9.446935 61.283707 -27.200068))
          (`self.EnterDigit` "4"))
        (:`4`
          (`self.AnimateButton` (`self.5`) (9.446888 61.283615 0.0))
          (`self.EnterDigit` "5"))
        (:`5`
          (`self.AnimateButton` (`self.6`) (9.446844 61.283527 27.19994))
          (`self.EnterDigit` "6"))
        (:`6`
          (`self.AnimateButton` (`self.7`) (31.046848 61.28363 -27.200012))
          (`self.EnterDigit` "7"))
        (:`7`
          (`self.AnimateButton` (`self.8`) (31.046803 61.283539 0.0))
          (`self.EnterDigit` "8"))
        (:`8`
          (`self.AnimateButton` (`self.9`) (31.046759 61.283436 27.199993))
          (`self.EnterDigit` "9"))))))

(event `AnimateButton`
  (params (Component :type "SceneComponent Object Reference") (StartLocation :type "Vector Structure"))
  (bind (_start_location_x _start_location_y _start_location_z) (`KismetMathLibrary.BreakVector` (`self.Start Location`)))
  ;[1 1 1] Animate button
  (set `self.CanPressButton` false)
  (bind (_direction _newtrack_0) (`Timeline|Timeline_0` :!via `PlayFromStart`)
    (:`Update`
      (bind _output_get (set `self.Start Location` StartLocation))
      (`SceneComponent.K2_SetRelativeLocation` Component (`KismetMathLibrary.VLerp` _output_get (`KismetMathLibrary.MakeVector` _start_location_x (- _start_location_y 56.0) _start_location_z) _newtrack_0) false false))
    (:`Finished`
      (set `self.CanPressButton` true))))

(event `EnterDigit`
  (params (Number :type Text))
  ;[1 1 1] Enter digit
  (switch `int` (`self.DigitIndex`)
    (:`0`
      (set `self.Digit1` Number)
      (set `self.DigitIndex` 1))
    (:`1`
      (set `self.Digit2` Number)
      (set `self.DigitIndex` 2))
    (:`2`
      (set `self.Digit3` Number)
      (set `self.DigitIndex` 3))
    (:`3`
      (set `self.Digit4` Number)
      (set `self.DigitIndex` 0)))
  (if (`self.Unlocked`)
    (`GameplayStatics.SpawnSoundAttached` "/Game/MyContent/Sounds/SW_KeypadButton.SW_KeypadButton" (`self.DefaultSceneRoot`) "None" (0.0 0.0 0.0) (struct) "KeepRelativeOffset" false 1.0 1.0 0.0 "/Game/MyContent/Sounds/Att_Object.Att_Object" null)
    (else
      (bind _result (`self.UpdateKeypadNumbers`))
      (if (== (`self.DigitIndex`) 0)
        (if (`KismetTextLibrary.EqualEqual_TextText` _result (`self.Combination`))
          (set `self.Unlocked` true)
          (`PrimitiveComponent.SetMaterial` (`self.Light`) 0 "/Game/MyContent/Materials/MI_Glow_Green.MI_Glow_Green")
          (`GameplayStatics.SpawnSoundAttached` "/Game/MyContent/Sounds/SW_Unlocked.SW_Unlocked" (`self.DefaultSceneRoot`) "None" (0.0 0.0 0.0) (struct) "KeepRelativeOffset" false 1.0 1.0 0.0 "/Game/MyContent/Sounds/Att_Object.Att_Object" null)
          (`self.ActivateReceiver`)
          (else
            (set `self.Locked` true)
            (`PrimitiveComponent.SetMaterial` (`self.Light`) 0 "/Game/MyContent/Materials/MI_Glow_red.MI_Glow_red")
            (`GameplayStatics.SpawnSoundAttached` "/Game/MyContent/Sounds/SW_Invalid.SW_Invalid" (`self.DefaultSceneRoot`) "None" (0.0 0.0 0.0) (struct) "KeepRelativeOffset" false 1.0 1.0 0.0 "/Game/MyContent/Sounds/Att_Object.Att_Object" null)
            (`KismetSystemLibrary.Delay` 1.0)
            (set `self.Digit1` "-")
            (set `self.Digit2` "-")
            (set `self.Digit3` "-")
            (set `self.Digit4` "-")
            (`self.UpdateKeypadNumbers`)
            (set `self.Locked` false)
            (`PrimitiveComponent.SetMaterial` (`self.Light`) 0 "/Engine/BasicShapes/BasicShapeMaterial.BasicShapeMaterial")))
        (else
          (`GameplayStatics.SpawnSoundAttached` "/Game/MyContent/Sounds/SW_KeypadButton.SW_KeypadButton" (`self.DefaultSceneRoot`) "None" (0.0 0.0 0.0) (struct) "KeepRelativeOffset" false 1.0 1.0 0.0 "/Game/MyContent/Sounds/Att_Object.Att_Object" null))))))

(fn `UserConstructionScript`)