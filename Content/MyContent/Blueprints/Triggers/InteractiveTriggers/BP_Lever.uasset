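; BP_Lever is an interactive lever trigger that toggles a receiver on and off.
; Each Interactwith event alternates through a FlipFlop between activating and deactivating the receiver, each with its own button sound.
; A timeline plays or reverses to swing the Cylinder between two angles, while Cylinder1 swaps between a glow material and a basic one to show the state.
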(event `/Game/MyContent/Blueprints/Interfaces/BPI_Interact.InteractWith`
  (params (FPS_Character :type "/Game/MyContent/Blueprints/Player/FirstPersonCharacter Object Reference"))
  (bind _returnvalue (`self.K2_GetActorLocation`))
  (`/Engine/EditorBlueprintResources/StandardMacros.FlipFlop`
    (:`A`
      (`self.ActivateReceiver`)
      (`GameplayStatics.PlaySoundAtLocation` "/Game/MyContent/Sounds/SW_UI_Button1.SW_UI_Button1" _returnvalue (struct) 0.6 1.0 0.0 "/Game/MyContent/Sounds/Att_Object.Att_Object" null null null)
      (`PrimitiveComponent.SetMaterial` (`self.Cylinder1`) 0 "/Game/MyContent/Materials/M_Glow.M_Glow")
      (bind (_direction _newtrack_0) (`Timeline|Timeline_0` :!label _label)
        (:`Update`
          (`SceneComponent.K2_SetRelativeRotation` (`self.Cylinder`) (`KismetMathLibrary.RLerp` (struct :`Pitch` 30.0) (struct :`Pitch` -30.0) _newtrack_0) false false))))
    (:`B`
      (`self.DeactivateReceiver`)
      (`GameplayStatics.PlaySoundAtLocation` "/Game/MyContent/Sounds/SW_UI_Button2.SW_UI_Button2" _returnvalue (struct) 0.6 1.0 0.0 "/Game/MyContent/Sounds/Att_Object.Att_Object" null null null)
      (`PrimitiveComponent.SetMaterial` (`self.Cylinder1`) 0 "/Engine/BasicShapes/BasicShapeMaterial.BasicShapeMaterial")
      (goto _label :!via `Reverse`))))

(fn `UserConstructionScript`
  (`parent.UserConstructionScript`))