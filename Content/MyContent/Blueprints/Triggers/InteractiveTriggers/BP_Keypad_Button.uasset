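; BP_Keypad_Button is an interactive keypad button that stores its label and animates when used.
; SetText saves the incoming text into the Number variable.
; Interactwith plays a timeline that lerps the Cube between zero and a small downward Z offset as a press motion, applied as an absolute world location rather than relative to the button.
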(event `/Game/MyContent/Blueprints/Interfaces/BPI_Widget.SetText`
  (params (Text :type Text))
  (set `self.Number` Text))

(event `/Game/MyContent/Blueprints/Interfaces/BPI_Interact.InteractWith`
  (params (FPS_Character :type "/Game/MyContent/Blueprints/FirstPersonCharacter Object Reference"))
  (bind (_direction _newtrack_0) (`Timeline|Timeline_0`)
    (:`Update`
      (`SceneComponent.K2_SetWorldLocation` (`self.Cube`) (`KismetMathLibrary.VLerp` (0.0 0.0 0.0) (0.0 0.0 -3.0) _newtrack_0) false false))))

(fn `UserConstructionScript`
  (`parent.UserConstructionScript`))