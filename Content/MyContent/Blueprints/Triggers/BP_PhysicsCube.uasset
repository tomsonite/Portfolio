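; BP_PhysicsCube is a physics cube that the player can pick up and drop, and that can activate weight pads.
; Each interaction flip-flops between grabbing the static mesh at its location with the FPS character's PhysicsHandle and releasing it.
; High angular damping is applied while held to resist spinning, then cleared on release.
; The ActivateWeightPad event calls ActivatePad on the pad passed to it.
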(event `/Game/MyContent/Blueprints/Interfaces/BPI_Interact.InteractWith`
  (params (FPS_Character :type "/Game/MyContent/Blueprints/Player/FirstPersonCharacter Object Reference"))
  (bind _staticmesh (`self.StaticMesh`))
  (`/Engine/EditorBlueprintResources/StandardMacros.FlipFlop`
    (:`A`
      (`PhysicsHandleComponent.GrabComponentAtLocation` (`/Game/MyContent/Blueprints/Player/FirstPersonCharacter.PhysicsHandle` FPS_Character) _staticmesh "None" (`SceneComponent.K2_GetComponentLocation` _staticmesh))
      (`PrimitiveComponent.SetAngularDamping` (`self.StaticMesh`) 100.0))
    (:`B`
      (`PhysicsHandleComponent.ReleaseComponent` (`/Game/MyContent/Blueprints/Player/FirstPersonCharacter.PhysicsHandle` FPS_Character))
      (`PrimitiveComponent.SetAngularDamping` (`self.StaticMesh`) 0.0))))

(event `/Game/MyContent/Blueprints/Interfaces/BPI_PhysicsObject.ActivateWeightPad`
  (params (WeightPad :type "/Game/MyContent/Blueprints/Triggers/BP_WeightPad Object Reference"))
  (`/Game/MyContent/Blueprints/Triggers/BP_WeightPad.ActivatePad` WeightPad))

(fn `UserConstructionScript`)