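; Sliding door receiver that opens when the player character enters its trigger box while it is unlocked and closes when they leave.
; A timeline fakes the slide by squashing the door's Scene component to near-zero Z scale, then reverses to close it.
; Activate unlocks the door, while Deactivate closes and locks it.
; A rect light shows green or red for the lock state, also set by the construction script.
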(event `self.Box.OnComponentBeginOverlap`
  (params (OverlappedComponent :type "PrimitiveComponent Object Reference") (OtherActor :type "Actor Object Reference") (OtherComp :type "PrimitiveComponent Object Reference") (OtherBodyIndex :type Integer) (bFromSweep :type Boolean) (SweepResult :type "HitResult Structure (by ref)"))
  (if (and (== OtherActor (`GameplayStatics.GetPlayerCharacter` 0)) (`self.Unlocked?`))
    (bind (_direction _newtrack_0) (`Timeline|Timeline_0` :!label _label)
      (:`Update`
        (`SceneComponent.SetRelativeScale3D` (`self.Scene`) (`KismetMathLibrary.VLerp` (1.0 1.0 1.0) (1.0 1.0 0.00029) _newtrack_0))))))

(event `CloseDoor`
  (goto _label :!via `Reverse`))

(event `self.Box.OnComponentEndOverlap`
  (params (OverlappedComponent :type "PrimitiveComponent Object Reference") (OtherActor :type "Actor Object Reference") (OtherComp :type "PrimitiveComponent Object Reference") (OtherBodyIndex :type Integer))
  (if (and (== OtherActor (`GameplayStatics.GetPlayerCharacter` 0)) (`self.Unlocked?`))
    (goto _label :!via `Reverse`)))

(event `/Game/MyContent/Blueprints/Interfaces/BPI_Receiver.Activate`
  (`self.Unlock?` true))

(event `/Game/MyContent/Blueprints/Interfaces/BPI_Receiver.Deactivate`
  (`self.CloseDoor`)
  (`self.Unlock?` false))

(fn `Unlock?`
  (params (`Unlocked?` :type Boolean))
  (bind _rectlight (`self.RectLight`))
  (bind _output_get (set `self.Unlocked?` `Unlocked?`))
  (if _output_get
    (`LightComponent.SetLightColor` _rectlight (struct :`G` 1.0 :`A` 1.0) true)
    (else
      (`LightComponent.SetLightColor` _rectlight (struct :`R` 1.0 :`A` 1.0) true))))

(fn `UserConstructionScript`
  (bind _rectlight (`self.RectLight`))
  (if (`self.Unlocked?`)
    (`LightComponent.SetLightColor` _rectlight (struct :`G` 1.0 :`A` 1.0) true)
    (else
      (`LightComponent.SetLightColor` _rectlight (struct :`R` 1.0 :`A` 1.0) true))))