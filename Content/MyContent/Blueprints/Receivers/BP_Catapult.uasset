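; BP_Catapult is a receiver actor that swings its arm, a Cube component, when activated.
; Activate plays a timeline that lerps the cube's relative pitch or yaw rotation through a throw arc, waits briefly, then plays a second timeline to return it.
; A CanActivate flag blocks retriggering until the return finishes.
; The launch is purely this rotation, with no impulse logic.
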(event `/Game/MyContent/Blueprints/Interfaces/BPI_Receiver.Activate`
  (if (`self.CanActivate`)
    (set `self.CanActivate` false)
    (bind (_direction _newtrack_0) (`Timeline|Timeline_0` :!via `PlayFromStart`)
      (:`Update`
        (`SceneComponent.K2_SetRelativeRotation` (`self.Cube`) (`KismetMathLibrary.RLerp` (struct :`Pitch` -30.0) (struct :`Pitch` 60.0) _newtrack_0) false false))
      (:`Finished`
        (`KismetSystemLibrary.Delay` 2.0)
        (bind (_direction_2 _newtrack_0_2) (`Timeline|Timeline_1` :!via `PlayFromStart`)
          (:`Update`
            (`SceneComponent.K2_SetRelativeRotation` (`self.Cube`) (`KismetMathLibrary.RLerp` (struct :`Pitch` 60.0) (struct :`Pitch` -30.0) _newtrack_0_2) false false))
          (:`Finished`
            (set `self.CanActivate` true)))))))

(fn `UserConstructionScript`
  (`parent.UserConstructionScript`))