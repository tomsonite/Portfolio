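; BP_SettingsActor is an actor that owns the pause menu and triggers settings initialization when play begins.
; On BeginPlay it creates and stores a W_PauseMenuContainer widget and calls its InitializeSettings without displaying it.
; The Pause input adds that widget to the viewport, switches to UI-only input, shows the cursor and centers it using the screen resolution from GameUserSettings.
; It neither pauses the game nor closes the menu.
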(event `self.ReceiveBeginPlay`
  (bind _returnvalue (`|CreateWidget` "/Game/MyContent/Widgets/W_PauseMenuContainer.W_PauseMenuContainer_C"))
  (bind _output_get (set `self.PauseMenu` _returnvalue))
  (`/Game/MyContent/Widgets/W_PauseMenuContainer.InitializeSettings` _output_get))

(event `InputAction|Pause`
  (params (Key :type "Key Structure"))
  (bind _returnvalue (`GameplayStatics.GetPlayerController` 0))
  (:`Pressed`
    (`UserWidget.AddToViewport` (`self.PauseMenu`) 0)
    (`WidgetBlueprintLibrary.SetInputMode_UIOnlyEx` _returnvalue (`self.PauseMenu`))
    (set `PlayerController.bShowMouseCursor` true _returnvalue)
    ;[1 1 1] move mouse to middle of screen
    (bind _returnvalue_2 (`GameUserSettings.GetGameUserSettings`))
    (bind (_returnvalue_x _returnvalue_y) (break `IntPoint` (`GameUserSettings.GetScreenResolution` _returnvalue_2)))
    (`PlayerController.SetMouseLocation` _returnvalue (/ _returnvalue_x 2) (/ _returnvalue_y 2))))

(fn `UserConstructionScript`)