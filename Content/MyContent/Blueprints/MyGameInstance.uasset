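; MyGameInstance is a game instance Blueprint that holds the save game object for the player's audio, controller, graphics and keyboard/mouse settings.
; SetSaveGame stores that object, which is supplied by the caller rather than loaded or created here.
; SaveSettings copies all four settings groups into it and writes it synchronously to a single save slot.
; GetSettings returns the same groups straight from the stored object, with no validity check.
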(event `/Game/MyContent/Blueprints/Interfaces/BPI_GameInstance.SaveSettings`
  (params (AudioSettings :type "/Game/MyContent/Blueprints/Structs/Struct_AudioSettings Structure") (ControllerSettings :type "/Game/MyContent/Blueprints/Structs/Struct_ControllerSettings Structure") (GraphicsSettings :type "/Game/MyContent/Blueprints/Structs/Struct_GraphicsSettings Structure") (KeyboardSettings :type "/Game/MyContent/Blueprints/Structs/Struct_KeyboardSettings Structure"))
  (bind _my_save_game (`self.My Save Game`))
  (set `/Game/MyContent/Blueprints/BP_MySaveGame.AudioSettings` AudioSettings _my_save_game)
  (set `/Game/MyContent/Blueprints/BP_MySaveGame.ControllerSettings` ControllerSettings _my_save_game)
  (set `/Game/MyContent/Blueprints/BP_MySaveGame.GraphicsSettings` GraphicsSettings _my_save_game)
  (set `/Game/MyContent/Blueprints/BP_MySaveGame.M&KBSettings` KeyboardSettings _my_save_game)
  (`GameplayStatics.SaveGameToSlot` (`self.My Save Game`) "saveslot"))

(event `/Game/MyContent/Blueprints/Interfaces/BPI_GameInstance.SetSaveGame`
  (params (MySaveGame :type "/Game/MyContent/Blueprints/BP_MySaveGame Object Reference"))
  (set `self.My Save Game` MySaveGame))

(fn `GetSettings`
  (returns (AudioSettings :type "/Game/MyContent/Blueprints/Structs/Struct_AudioSettings Structure") (ControllerSettings :type "/Game/MyContent/Blueprints/Structs/Struct_ControllerSettings Structure") (GraphicsSettings :type "/Game/MyContent/Blueprints/Structs/Struct_GraphicsSettings Structure") (KeyboardSettings :type "/Game/MyContent/Blueprints/Structs/Struct_KeyboardSettings Structure"))
  (bind _my_save_game (`self.My Save Game`))
  (return (`/Game/MyContent/Blueprints/BP_MySaveGame.AudioSettings` _my_save_game) (`/Game/MyContent/Blueprints/BP_MySaveGame.ControllerSettings` _my_save_game) (`/Game/MyContent/Blueprints/BP_MySaveGame.GraphicsSettings` _my_save_game) (`/Game/MyContent/Blueprints/BP_MySaveGame.M&KBSettings` _my_save_game)))